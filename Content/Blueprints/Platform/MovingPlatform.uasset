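; Moving platform Blueprint that ping-pongs a static mesh between two offsets from its starting world location.
; StartMovement plays a timeline that lerps the mesh between PlatformStart and PlatformEnd, flipping direction after a short pause at each end.
; EndMovement stops the timeline, while ReverseTime also sets IsReversed to suppress position updates.
; UnReverse clears that flag and reissues playback in the current direction only if the timeline is still playing.
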(event Custom|StartMovement
  (bind (_direction _driver) (Timeline|LoweringTimeline Play)
    (:Update
      (if (not (Variables|Default|GetIsReversed))
        (Transformation|SetWorldLocation (Variables|Debug|GetStaticMeshComponent) (+ (Variables|WalkwaySetup|GetOriginal_loc) (Math|Vector|Lerp(Vector) (Variables|WalkwaySetup|GetPlatformStart) (Variables|WalkwaySetup|GetPlatformEnd) _driver)) false false)))
    (:Finished
      (Utilities|FlowControl|Delay 0.5)
      (if (Utilities|Enum|Equal(Enum) _direction "Forward")
        (Timeline|LoweringTimeline Reverse)
        (else
          (Timeline|LoweringTimeline Play))))))

(event Custom|EndMovement
  (bind (_direction _driver) (Timeline|LoweringTimeline Stop)
    (:Update
      (if (not (Variables|Default|GetIsReversed))
        (Transformation|SetWorldLocation (Variables|Debug|GetStaticMeshComponent) (+ (Variables|WalkwaySetup|GetOriginal_loc) (Math|Vector|Lerp(Vector) (Variables|WalkwaySetup|GetPlatformStart) (Variables|WalkwaySetup|GetPlatformEnd) _driver)) false false)))
    (:Finished
      (Utilities|FlowControl|Delay 0.5)
      (if (Utilities|Enum|Equal(Enum) _direction "Forward")
        (Timeline|LoweringTimeline Reverse)
        (else
          (Timeline|LoweringTimeline Play))))))

(event Custom|ReverseTime
  (Variables|Default|SetIsReversed true)
  (bind (_direction _driver) (Timeline|LoweringTimeline Stop)
    (:Update
      (if (not (Variables|Default|GetIsReversed))
        (Transformation|SetWorldLocation (Variables|Debug|GetStaticMeshComponent) (+ (Variables|WalkwaySetup|GetOriginal_loc) (Math|Vector|Lerp(Vector) (Variables|WalkwaySetup|GetPlatformStart) (Variables|WalkwaySetup|GetPlatformEnd) _driver)) false false)))
    (:Finished
      (Utilities|FlowControl|Delay 0.5)
      (if (Utilities|Enum|Equal(Enum) _direction "Forward")
        (Timeline|LoweringTimeline Reverse)
        (else
          (Timeline|LoweringTimeline Play))))))

(event Custom|UnReverse
  (Variables|Default|SetIsReversed false)
  (if (Audio|Components|Audio|IsPlaying (Variables|Default|GetLoweringTimeline))
    (if (Utilities|Enum|Equal(Enum) (stale _direction) "Forward")
      (bind (_direction _driver) (Timeline|LoweringTimeline Play)
        (:Update
          (if (not (Variables|Default|GetIsReversed))
            (Transformation|SetWorldLocation (Variables|Debug|GetStaticMeshComponent) (+ (Variables|WalkwaySetup|GetOriginal_loc) (Math|Vector|Lerp(Vector) (Variables|WalkwaySetup|GetPlatformStart) (Variables|WalkwaySetup|GetPlatformEnd) _driver)) false false)))
        (:Finished
          (Utilities|FlowControl|Delay 0.5)
          (if (Utilities|Enum|Equal(Enum) _direction "Forward")
            (Timeline|LoweringTimeline Reverse)
            (else
              (Timeline|LoweringTimeline Play)))))
      (else
        (Timeline|LoweringTimeline Reverse)))))

(event EventBeginPlay
  (Variables|WalkwaySetup|SetOriginal_loc (Transformation|GetWorldLocation (Variables|Debug|GetStaticMeshComponent))))

(fn ConstructionScript)