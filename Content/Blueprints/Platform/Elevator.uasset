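; Elevator platform, or walkway, that moves its static mesh between two offsets from its starting location.
; LowerWalkway and RaiseWalkway play and reverse one timeline, whose driver lerps the offset.
; Save records timeline position and direction in capped arrays, and Play restores and pops the latest entry for rewind-style playback, resuming motion if mid-travel.
; Movement sound logic is present but disconnected, and Tick is empty.
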(event Custom|LowerWalkway
  ;[1 1 1] Lower the walkway and raise it
  (bind (_direction _driver) (Timeline|LoweringTimeline Play)
    (:Update
      (Transformation|SetWorldLocation (Variables|Debug|GetStaticMeshComponent) (+ (Variables|WalkwaySetup|GetOriginal_loc) (Math|Vector|Lerp(Vector) (Variables|WalkwaySetup|GetWalkwayUp) (Variables|WalkwaySetup|GetWalkwayDown) _driver)) false false)
      (Variables|Default|SetisMoving true))
    (:Finished
      (Variables|Default|SetisMoving false))))

(event Custom|RaiseWalkway
  ;[1 1 1] Lower the walkway and raise it
  (bind (_direction _driver) (Timeline|LoweringTimeline Reverse)
    (:Update
      (Transformation|SetWorldLocation (Variables|Debug|GetStaticMeshComponent) (+ (Variables|WalkwaySetup|GetOriginal_loc) (Math|Vector|Lerp(Vector) (Variables|WalkwaySetup|GetWalkwayUp) (Variables|WalkwaySetup|GetWalkwayDown) _driver)) false false)
      (Variables|Default|SetisMoving true))
    (:Finished
      (Variables|Default|SetisMoving false))))

(event EventTick
  (params (DeltaSeconds :type Float%20%28single-precision%29)))

(event EventSave
  (params (limit :type Integer))
  (bind _timelinepositions (Variables|Default|GetTimelinePositions))
  (bind _directions (Variables|Default|GetDirections))
  ;[1 1 1] Save position and direction
  (if (>= limit (Utilities|Array|Length _timelinepositions))
    (Utilities|Array|Add (Variables|Default|GetTimelinePositions) (Components|Timeline|GetPlaybackPosition (Variables|Default|GetLoweringTimeline)))
    (Utilities|Array|Add _directions (stale Custom|LowerWalkway _direction))
    (else
      (Utilities|Array|RemoveIndex _timelinepositions)
      (Utilities|Array|RemoveIndex _directions))))

(event EventPlay
  (bind _timelinepositions (Variables|Default|GetTimelinePositions))
  (bind _directions (Variables|Default|GetDirections))
  (bind _loweringtimeline (Variables|Default|GetLoweringTimeline))
  (bind _directions_2 (Variables|Default|GetDirections))
  (bind _returnvalue (Utilities|Array|LastIndex _timelinepositions))
  (bind _item (Utilities|Array|Get(acopy) _timelinepositions _returnvalue))
  ;[1 1 1] Restore position and direction
  (if (> (Utilities|Array|Length _timelinepositions) 1)
    (Components|Timeline|SetPlaybackPosition (Variables|Default|GetLoweringTimeline) _item false true)
    (Utilities|FlowControl|Sequence
      (:then_0
        (if (not (or (== _item 0.0) (== _item 1.0)))
          (if (Utilities|Enum|Equal(Enum) (Utilities|Array|Get(acopy) _directions_2 (Utilities|Array|LastIndex _directions_2)) "Forward")
            (Audio|Components|Audio|Play _loweringtimeline)
            (else
              (Utilities|String|Reverse _loweringtimeline)))))
      (:then_1
        (Utilities|Array|RemoveIndex (Variables|Default|GetTimelinePositions) _returnvalue)
        (Utilities|Array|RemoveIndex _directions (Utilities|Array|LastIndex _directions))))))

(event EventBeginPlay
  ;[1 1 1] Set original location
  (Variables|WalkwaySetup|SetOriginal_loc (Transformation|GetWorldLocation (Variables|Debug|GetStaticMeshComponent))))

(fn ConstructionScript)