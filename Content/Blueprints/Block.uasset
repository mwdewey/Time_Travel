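; Block is an actor that a character can pick up and drop by interacting with it.
; InteractedWith toggles the held state, storing the interacting character on pickup and switching the mesh's gravity off while held, back on when dropped.
; While held, Tick moves the actor each frame to a fixed distance along that character's forward vector, with no physics handle or attachment.
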(event Custom|InteractedWith
  (params (Character :type Actor%20Object%20Reference))
  (bind _staticmeshcomponent (Variables|Debug|GetStaticMeshComponent))
  (if (Variables|Default|GetIsUp)
    (Variables|Default|SetIsUp false)
    (Physics|SetEnableGravity _staticmeshcomponent true)
    (else
      (Variables|Default|SetPlayerParent Character)
      (Variables|Default|SetIsUp true)
      (Physics|SetEnableGravity _staticmeshcomponent false))))

(event EventTick
  (params (DeltaSeconds :type Float%20%28single-precision%29))
  (bind _playerparent (Variables|Default|GetPlayerParent))
  (if (Variables|Default|GetIsUp)
    (Transformation|SetActorLocationAndRotation (+ (* (Transformation|GetActorForwardVector _playerparent) 1.5e+02) (Transformation|GetActorLocation _playerparent)) "0, 0, 0")))

(fn ConstructionScript)