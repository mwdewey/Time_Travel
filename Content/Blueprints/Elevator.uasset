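; Elevator actor that lowers and raises a walkway mesh through LowerWalkway and RaiseWalkway events.
; BeginPlay caches the mesh's world location as the origin for the movement.
; LoweringTimeline plays forward to lower and reverses to raise, with its Driver track blending between the WalkwayUp and WalkwayDown offsets added to that origin, without sweeping.
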(event Custom|LowerWalkway
  (bind _driver (Timeline|LoweringTimeline Play)
    (:Update
      (Transformation|SetWorldLocation (Variables|Debug|GetStaticMeshComponent) (+ (Variables|WalkwaySetup|GetOriginal_loc) (Math|Vector|Lerp(Vector) (Variables|WalkwaySetup|GetWalkwayUp) (Variables|WalkwaySetup|GetWalkwayDown) _driver)) false false))))

(event Custom|RaiseWalkway
  (bind _driver (Timeline|LoweringTimeline Reverse)
    (:Update
      (Transformation|SetWorldLocation (Variables|Debug|GetStaticMeshComponent) (+ (Variables|WalkwaySetup|GetOriginal_loc) (Math|Vector|Lerp(Vector) (Variables|WalkwaySetup|GetWalkwayUp) (Variables|WalkwaySetup|GetWalkwayDown) _driver)) false false))))

(event EventBeginPlay
  (Variables|WalkwaySetup|SetOriginal_loc (Transformation|GetWorldLocation (Variables|Debug|GetStaticMeshComponent))))

(fn ConstructionScript)