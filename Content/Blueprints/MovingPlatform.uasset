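; Moving platform Blueprint that shifts its static mesh between two offsets from where it began play.
; BeginPlay caches the mesh's world location, and StartMovement plays a looping timeline whose Driver value blends PlatformStart to PlatformEnd.
; Each update adds that offset to the cached location and sets it without sweep.
; EndMovement only turns looping off, so the current cycle finishes before the platform stops.
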(event Custom|StartMovement
  (Components|Timeline|SetLooping (Variables|Default|GetLoweringTimeline) true)
  (bind _driver (Timeline|LoweringTimeline Play)
    (:Update
      (Transformation|SetWorldLocation (Variables|Debug|GetStaticMeshComponent) (+ (Variables|WalkwaySetup|GetOriginal_loc) (Math|Vector|Lerp(Vector) (Variables|WalkwaySetup|GetPlatformStart) (Variables|WalkwaySetup|GetPlatformEnd) _driver)) false false))))

(event Custom|EndMovement
  (Components|Timeline|SetLooping (Variables|Default|GetLoweringTimeline) false))

(event EventBeginPlay
  (Variables|WalkwaySetup|SetOriginal_loc (Transformation|GetWorldLocation (Variables|Debug|GetStaticMeshComponent))))

(fn ConstructionScript)