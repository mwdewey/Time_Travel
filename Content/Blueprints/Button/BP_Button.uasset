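; BP_Button is a pressure button that is pushed down while something overlaps its TriggerBox and released when the overlap ends.
; Begin and end overlap, with no actor filter, call ButtonPushed and ButtonReleased, then set IsDown on the ButtonAnim instance.
; A timeline, played on press and reversed on release, lerps the Collider between up and down offsets from its BeginPlay location.
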(event OnComponentBeginOverlap(TriggerBox)
  (params (OtherActor :type Actor%20Object%20Reference) (OtherComp :type Primitive%20Component%20Object%20Reference) (OtherBodyIndex :type Integer) (bFromSweep :type Boolean) (SweepResult :type Hit%20Result%20Structure%20%28by%20ref%29))
  ;[1 1 1] Push down button
  (Default|CallButtonPushed)
  (bind _asbutton_anim (Utilities|Casting|CastToButtonAnim (Components|SkeletalMesh|GetAnimInstance (Variables|Components|GetButton))))
  (Variables|/Game/Blueprints/Button/ButtonAnim.ButtonAnim_C|SetIsDown _asbutton_anim true)
  (bind _driver (Timeline|Timeline_0 Play)
    (:Update
      (Transformation|SetWorldLocation (Variables|Components|GetCollider) (+ (Variables|ButtonSetup|GetOriginalLoc) (Math|Vector|Lerp(Vector) (Variables|ButtonSetup|GetButtonUp) (Variables|ButtonSetup|GetButtonDown) _driver)) false false))))

(event OnComponentEndOverlap(TriggerBox)
  (params (OtherActor :type Actor%20Object%20Reference) (OtherComp :type Primitive%20Component%20Object%20Reference) (OtherBodyIndex :type Integer))
  ;[1 1 1] Push down button
  (Default|CallButtonReleased)
  (bind _asbutton_anim (Utilities|Casting|CastToButtonAnim (Components|SkeletalMesh|GetAnimInstance (Variables|Components|GetButton))))
  (Variables|/Game/Blueprints/Button/ButtonAnim.ButtonAnim_C|SetIsDown _asbutton_anim false)
  (bind _driver (Timeline|Timeline_0 Reverse)
    (:Update
      (Transformation|SetWorldLocation (Variables|Components|GetCollider) (+ (Variables|ButtonSetup|GetOriginalLoc) (Math|Vector|Lerp(Vector) (Variables|ButtonSetup|GetButtonUp) (Variables|ButtonSetup|GetButtonDown) _driver)) false false))))

(event EventBeginPlay
  (Variables|ButtonSetup|SetOriginalLoc (Transformation|GetWorldLocation (Variables|Components|GetCollider))))

(fn ConstructionScript)