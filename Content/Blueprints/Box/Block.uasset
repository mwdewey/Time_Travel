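; Block is an interactable physics box that the player can pick up and carry, with support for rewinding its movement.
; Interaction toggles carrying and gravity; Tick sweeps it ahead of the carrier and drops it beyond a distance threshold.
; Save records transforms in a capped history, and Play teleports through them newest to oldest.
; Highlight and Unhighlight toggle a highlight component's visibility.
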(event Custom|InteractedWith
  (params (Character :type Actor%20Object%20Reference))
  ;[1 1 1] Begin or end parenting when interacted with
  (if (Variables|Default|GetIsUp)
    (Variables|Default|SetIsUp false)
    (else
      (Variables|Default|SetPlayerParent Character)
      (Variables|Default|SetIsUp true)))
  (Physics|SetEnableGravity (Variables|Debug|GetStaticMeshComponent) (not (Variables|Default|GetIsUp))))

(event EventUnhighlight
  ;[1 1 1] Highlighting
  (Rendering|SetVisibility (Variables|Default|GetHighlightedBlock) false false))

(event EventHighlight
  ;[1 1 1] Highlighting
  (Rendering|SetVisibility (Variables|Default|GetHighlightedBlock) true false))

(event EventSave
  (params (limit :type Integer))
  (bind _temptransformarray (Variables|Default|GettempTransformArray))
  (Variables|Default|SetFrameLimit limit)
  (Utilities|Array|Add _temptransformarray (Transformation|GetActorTransform))
  (if (> (Utilities|Array|Length _temptransformarray) (Variables|Default|GetFrameLimit))
    (Utilities|Array|RemoveIndex _temptransformarray)))

(event EventTick
  (params (DeltaSeconds :type Float%20%28single-precision%29))
  (bind _playerparent (Variables|Default|GetPlayerParent))
  (bind _returnvalue (Transformation|GetActorLocation _playerparent))
  ;[1 1 1] Update position based on parent
  (if (Variables|Default|GetIsUp)
    ;[1 1 1] Drop the block if too far away from player
    (Math|Float|CompareFloat (Math|Vector|VectorLength (- _returnvalue (Transformation|GetWorldLocation (Variables|Debug|GetStaticMeshComponent)))) 2e+02
      (:>
        ;[1 1 1] Begin or end parenting when interacted with
        (Variables|Default|SetIsUp false)
        (Physics|SetEnableGravity (Variables|Debug|GetStaticMeshComponent) (not (Variables|Default|GetIsUp))))
      (:==
        (bind _sweephitresult (Transformation|SetActorLocationAndRotation (+ (* (Transformation|GetActorForwardVector _playerparent) 1.5e+02) _returnvalue) "0, 0, 0" true :!label _label))
        (if (== _playerparent (.HitActor (Collision|BreakHitResult _sweephitresult)))
          (Utilities|FlowControl|FlipFlop
            (:A
              (goto _label)))))
      (:<
        (goto _label)))))

(event EventPlay
  (bind _temptransformarray (Variables|Default|GettempTransformArray))
  (bind _returnvalue (Utilities|Array|LastIndex _temptransformarray))
  (bind _item (Utilities|Array|Get(acopy) _temptransformarray _returnvalue))
  (Transformation|SetActorTransform _item false true)
  (if (not (== _returnvalue 0))
    (Utilities|Array|RemoveItem _temptransformarray _item)))

(fn ConstructionScript)