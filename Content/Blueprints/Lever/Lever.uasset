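; Lever actor that toggles between on and off and notifies listeners, such as a walkway, of its state.
; LeverToggled plays or reverses the ArmSwing timeline based on its current direction, lerping the arm's relative location and rotation.
; LeverOff fires as soon as switch-off begins, while LeverOn waits until the forward swing finishes.
; Highlight and Unhighlight show or hide separate highlighted base and arm components.
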(event Custom|LeverToggled
  (bind _leverarm (Variables|Default|GetLeverArm))
  ;[1 1 1] Notify that the lever is off as soon as pulled
  (if (Utilities|Enum|Equal(Enum) (stale _direction) "Backward")
    (bind (_direction _driver) (Timeline|ArmSwing Play)
      (:Update
        ;[1 1 1] Set the Rotation and Location
        (Transformation|SetRelativeLocation _leverarm (Math|Vector|Lerp(Vector) (Variables|Default|GetLocationOff) (Variables|Default|GetLocationOn) _driver) false false)
        (Transformation|SetRelativeRotation _leverarm (Math|Rotator|Lerp(Rotator) (Variables|Default|GetRotationOff) (Variables|Default|GetRotationOn) _driver) false false))
      (:Finished
        ;[1 1 1] Notify the walkway when the lever is on
        (if (not (Utilities|Enum|Equal(Enum) _direction "Backward"))
          (Default|CallLeveron))))
    (else
      (Default|CallLeverOff)
      (Timeline|ArmSwing Reverse))))

(event EventHighlight
  ;[1 1 1] Highlighting
  (Rendering|SetVisibility (Variables|Default|GetBaseHighlighted) true false)
  (Rendering|SetVisibility (Variables|Default|GetArmHighlighted) true false))

(event EventUnhighlight
  ;[1 1 1] Highlighting
  (Rendering|SetVisibility (Variables|Default|GetBaseHighlighted) false false)
  (Rendering|SetVisibility (Variables|Default|GetArmHighlighted) false false))

(fn ConstructionScript)