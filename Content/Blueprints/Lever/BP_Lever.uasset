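; BP_Lever is a toggleable lever actor that announces its on and off state to other objects.
; LeverToggled flips IsActive, fires the matching LeverOn or LeverOff dispatcher, and sets IsOn on the LeverAnim instances of both meshes.
; Highlighting uses a second mesh, LeverHighlighted, which Highlight and Unhighlight show or hide while it mirrors the main lever's animation.
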(event Custom|LeverToggled
  (bind _leverhighlighted (Variables|Default|GetLeverHighlighted))
  (bind _lever (Variables|Default|GetLever))
  (bind _returnvalue (Components|SkeletalMesh|GetAnimInstance _lever))
  (bind _returnvalue_2 (Components|SkeletalMesh|GetAnimInstance _leverhighlighted))
  ;[1 1 1] Notify that the lever is off as soon as pulled
  (if (Variables|Default|GetIsActive)
    (Default|CallLeverOff)
    (bind _aslever_anim (Utilities|Casting|CastToLeverAnim _returnvalue))
    (Variables|/Game/Blueprints/Lever/LeverAnim.LeverAnim_C|SetIsOn _aslever_anim false)
    (bind _aslever_anim_2 (Utilities|Casting|CastToLeverAnim _returnvalue_2))
    (Variables|/Game/Blueprints/Lever/LeverAnim.LeverAnim_C|SetIsOn _aslever_anim_2 false)
    (Variables|Default|SetIsActive false)
    (else
      (Default|CallLeveron)
      (bind _aslever_anim_3 (Utilities|Casting|CastToLeverAnim _returnvalue))
      (Variables|/Game/Blueprints/Lever/LeverAnim.LeverAnim_C|SetIsOn _aslever_anim_3 true)
      (bind _aslever_anim_4 (Utilities|Casting|CastToLeverAnim _returnvalue_2))
      (Variables|/Game/Blueprints/Lever/LeverAnim.LeverAnim_C|SetIsOn _aslever_anim_4 true)
      (Variables|Default|SetIsActive true))))

(event EventHighlight
  ;[1 1 1] Highlighting
  (Rendering|SetVisibility (Variables|Default|GetLeverHighlighted) true false))

(event EventUnhighlight
  ;[1 1 1] Highlighting
  (Rendering|SetVisibility (Variables|Default|GetLeverHighlighted) false false))

(fn ConstructionScript)