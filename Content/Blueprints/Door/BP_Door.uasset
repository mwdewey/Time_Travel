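; BP_Door is a door actor with Open and Close events that keep an animated door and its collider in step.
; Each event sets the IsClosed flag on the door's BPANIM_Door animation Blueprint and plays or reverses a shared timeline.
; The timeline moves the separate collider between DoorDown and DoorUp offsets from its world location saved at BeginPlay, without sweeping.
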(event Custom|Open
  (bind _asbpanim_door (Utilities|Casting|CastToBPANIM_Door (Components|SkeletalMesh|GetAnimInstance (Variables|Default|GetDoor))))
  (Variables|/Game/Blueprints/Door/BPANIM_Door.BPANIM_Door_C|SetIsClosed _asbpanim_door false)
  (bind _driver (Timeline|Timeline_0 Play)
    (:Update
      (Transformation|SetWorldLocation (Variables|Default|GetCollider) (+ (Variables|DoorSetup|GetOriginalLoc) (Math|Vector|Lerp(Vector) (Variables|DoorSetup|GetDoorDown) (Variables|DoorSetup|GetDoorUp) _driver)) false false))))

(event Custom|Close
  (bind _asbpanim_door (Utilities|Casting|CastToBPANIM_Door (Components|SkeletalMesh|GetAnimInstance (Variables|Default|GetDoor))))
  (Variables|/Game/Blueprints/Door/BPANIM_Door.BPANIM_Door_C|SetIsClosed _asbpanim_door true)
  (bind _driver (Timeline|Timeline_0 Reverse)
    (:Update
      (Transformation|SetWorldLocation (Variables|Default|GetCollider) (+ (Variables|DoorSetup|GetOriginalLoc) (Math|Vector|Lerp(Vector) (Variables|DoorSetup|GetDoorDown) (Variables|DoorSetup|GetDoorUp) _driver)) false false))))

(event EventBeginPlay
  (Variables|DoorSetup|SetOriginalLoc (Transformation|GetWorldLocation (Variables|Default|GetCollider))))

(fn ConstructionScript)