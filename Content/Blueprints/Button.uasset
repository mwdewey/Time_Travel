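; Pressure button actor that sinks when something overlaps its trigger box and signals pushed and released events.
; Overlap plays a timeline that lerps the static mesh's relative location from up to down, firing ButtonPushed only when the forward press completes.
; End overlap fires ButtonReleased immediately, even after a partial press, and reverses the timeline to raise the mesh.
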(event OnComponentBeginOverlap(TriggerBox)
  (params (OtherActor :type Actor%20Object%20Reference) (OtherComp :type Primitive%20Component%20Object%20Reference) (OtherBodyIndex :type Integer) (bFromSweep :type Boolean) (SweepResult :type Hit%20Result%20Structure%20%28by%20ref%29))
  (bind (_direction _driver) (Timeline|DepressTimeline Play)
    (:Update
      (Transformation|SetRelativeLocation (Variables|Default|GetStaticMesh) (Math|Vector|Lerp(Vector) (Variables|ButtonSetup|GetButtonUp) (Variables|ButtonSetup|GetButtonDown) _driver) false false))
    (:Finished
      (if (Utilities|Enum|Equal(Enum) _direction "Forward")
        (Default|CallButtonPushed)))))

(event OnComponentEndOverlap(TriggerBox)
  (params (OtherActor :type Actor%20Object%20Reference) (OtherComp :type Primitive%20Component%20Object%20Reference) (OtherBodyIndex :type Integer))
  (Default|CallButtonReleased)
  (bind (_direction _driver) (Timeline|DepressTimeline Reverse)
    (:Update
      (Transformation|SetRelativeLocation (Variables|Default|GetStaticMesh) (Math|Vector|Lerp(Vector) (Variables|ButtonSetup|GetButtonUp) (Variables|ButtonSetup|GetButtonDown) _driver) false false))
    (:Finished
      (if (Utilities|Enum|Equal(Enum) _direction "Forward")
        (Default|CallButtonPushed)))))

(fn ConstructionScript)